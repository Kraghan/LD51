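; BP_EndPortal is a level exit that loads NextLevel when a player-controlled BP_Player overlaps its trigger while open.
; It opens when every linked button is active, or immediately if none are linked, but closes only once all are inactive.
; Open and close events toggle the plane's visibility and portal audio, with playback starting after a delay if still open.
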(event OnComponentBeginOverlap(Trigger)
  (params (OverlappedComponent :type Primitive%20Component%20Object%20Reference) (OtherActor :type Actor%20Object%20Reference) (OtherComp :type Primitive%20Component%20Object%20Reference) (OtherBodyIndex :type Integer) (bFromSweep :type Boolean) (SweepResult :type Hit%20Result%20Structure%20%28by%20ref%29))
  (if (Variables|Default|GetIsOpen)
    (bind _asbp_player (Utilities|Casting|CastToBP_Player OtherActor))
    (Utilities|Casting|CastToBP_PlayerController (Pawn|GetController _asbp_player))
    (Default|CallOnPortalReached)
    (Game|OpenLevel(byObjectReference) (Variables|Default|GetNextLevel))))

(event Custom|OnPortalOpen_Event
  (Rendering|SetVisibility (Variables|Default|GetPlane) true false)
  (Variables|Default|SetIsOpen true)
  (Audio|PlaySound2D "/Game/Sound/portal.portal" 1.0 1.0 0.0 0 0)
  (Utilities|FlowControl|Delay 4.0)
  (if (Variables|Default|GetIsOpen)
    (Audio|Components|Audio|Play (Variables|Default|Getportal) 0.0)))

(event Custom|OnPortalClose_Event
  (Rendering|SetVisibility (Variables|Default|GetPlane) false false)
  (Variables|Default|SetIsOpen false)
  (Audio|Components|Audio|Stop (Variables|Default|Getportal)))

(event EventBeginPlay
  (for _array_element (Variables|Default|GetButtonsLinked)
    (EventDispatchers|BindEventtoOnButtonActivated _array_element (EventDispatchers|CreateEvent :!event OnButtonon))
    (EventDispatchers|BindEventtoOnButtonDeactivated _array_element (EventDispatchers|CreateEvent :!event OnButtonOff)))
  (EventDispatchers|BindEventtoOnPortalOpen (EventDispatchers|CreateEvent :!event Custom|OnPortalOpen_Event))
  (EventDispatchers|BindEventtoOnPortalClose (EventDispatchers|CreateEvent :!event Custom|OnPortalClose_Event))
  (Rendering|SetVisibility (Variables|Default|GetPlane) false false)
  (if (Utilities|Array|IsEmpty (Variables|Default|GetButtonsLinked))
    (CallFunction|OnButtonon)))

(fn ConstructionScript)

(fn OnButtonon
  (params (Button :type BP%20Button%20Object%20Reference))
  (for _array_element (Variables|Default|GetButtonsLinked)
    (if (not (Default|IsActive _array_element))
      (return)))
  (Default|CallOnPortalOpen))

(fn OnButtonOff
  (params (Button :type BP%20Button%20Object%20Reference))
  (for _array_element (Variables|Default|GetButtonsLinked)
    (if (Default|IsActive _array_element)
      (return)))
  (Default|CallOnPortalClose))