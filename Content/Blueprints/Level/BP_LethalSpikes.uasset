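; BP_LethalSpikes is a spike trap that raises spikes and kills players who touch its lethal volume.
; A player entering TriggerTrap is tracked in InTrigger, and after an activation delay a timeline drives the spikes' relative Z.
; The timeline reverses whenever a player leaves the trigger, or when it finishes with InTrigger empty.
; A separate TriggerLethal overlap calls Die on the player, independent of the timeline state.
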(event OnComponentBeginOverlap(TriggerTrap)
  (params (OverlappedComponent :type Primitive%20Component%20Object%20Reference) (OtherActor :type Actor%20Object%20Reference) (OtherComp :type Primitive%20Component%20Object%20Reference) (OtherBodyIndex :type Integer) (bFromSweep :type Boolean) (SweepResult :type Hit%20Result%20Structure%20%28by%20ref%29))
  (bind _spikes (Variables|Default|GetSpikes))
  (bind _relativelocation (Variables|/Script/Engine.SceneComponent|GetRelativeLocation _spikes))
  (bind _asbp_player (Utilities|Casting|CastToBP_Player OtherActor))
  (Utilities|Array|AddUnique (Variables|Default|GetInTrigger) _asbp_player)
  (Utilities|FlowControl|Delay (Variables|Default|GetActivationDelay))
  (bind _newtrack_0 (Timeline|Timeline_0 Play)
    (:Update
      (Transformation|SetRelativeLocation _spikes (Math|Vector|MakeVector (.x _relativelocation) (.y _relativelocation) _newtrack_0) false false))
    (:Finished
      (if (Utilities|Array|IsEmpty (Variables|Default|GetInTrigger))
        (Timeline|Timeline_0 Reverse)))))

(event OnComponentEndOverlap(TriggerTrap)
  (params (OverlappedComponent :type Primitive%20Component%20Object%20Reference) (OtherActor :type Actor%20Object%20Reference) (OtherComp :type Primitive%20Component%20Object%20Reference) (OtherBodyIndex :type Integer))
  (bind _spikes (Variables|Default|GetSpikes))
  (bind _relativelocation (Variables|/Script/Engine.SceneComponent|GetRelativeLocation _spikes))
  (bind _asbp_player (Utilities|Casting|CastToBP_Player OtherActor))
  (Utilities|Array|RemoveItem (Variables|Default|GetInTrigger) _asbp_player)
  (bind _newtrack_0 (Timeline|Timeline_0 Reverse)
    (:Update
      (Transformation|SetRelativeLocation _spikes (Math|Vector|MakeVector (.x _relativelocation) (.y _relativelocation) _newtrack_0) false false))
    (:Finished
      (if (Utilities|Array|IsEmpty (Variables|Default|GetInTrigger))
        (Timeline|Timeline_0 Reverse)))))

(event OnComponentBeginOverlap(TriggerLethal)
  (params (OverlappedComponent :type Primitive%20Component%20Object%20Reference) (OtherActor :type Actor%20Object%20Reference) (OtherComp :type Primitive%20Component%20Object%20Reference) (OtherBodyIndex :type Integer) (bFromSweep :type Boolean) (SweepResult :type Hit%20Result%20Structure%20%28by%20ref%29))
  (bind _asbp_player (Utilities|Casting|CastToBP_Player OtherActor))
  (Default|Die _asbp_player "NewEnumerator2"))

(event EventBeginPlay)

(event Collision|EventActorBeginOverlap
  (params (OtherActor :type Actor%20Object%20Reference)))

(event EventTick
  (params (DeltaSeconds :type Float%20%28single-precision%29)))

(fn ConstructionScript)