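; Spike trap actor whose spikes are driven by a linked button.
; On BeginPlay it binds to the linked button's activated and deactivated events.
; Activation plays the SpikeElevation timeline, which sets the spikes' relative Z location, and deactivation reverses it.
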(event Custom|OnButtonActivated
  (params (Button :type BP%20Button%20Object%20Reference))
  (bind _newtrack_0 (Timeline|SpikeElevation Play)
    (:Update
      (Transformation|SetRelativeLocation (Variables|Default|GetSpikes) (Math|Vector|MakeVector 0.0 0.0 _newtrack_0) false false))))

(event Custom|OnButtonDeactivated
  (params (Button :type BP%20Button%20Object%20Reference))
  (bind _newtrack_0 (Timeline|SpikeElevation Reverse)
    (:Update
      (Transformation|SetRelativeLocation (Variables|Default|GetSpikes) (Math|Vector|MakeVector 0.0 0.0 _newtrack_0) false false))))

(event EventBeginPlay
  (EventDispatchers|BindEventtoOnButtonActivated (Variables|Default|GetLinkedButton) (EventDispatchers|CreateEvent :!event Custom|OnButtonActivated))
  (EventDispatchers|BindEventtoOnButtonDeactivated (Variables|Default|GetLinkedButton) (EventDispatchers|CreateEvent :!event Custom|OnButtonDeactivated)))

(fn ConstructionScript)