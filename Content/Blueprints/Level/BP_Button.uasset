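; BP_Button is a pressure button actor that stays active while one or more BP_Player characters stand on it.
; Sphere overlaps track players in CharaOnButton, firing OnButtonActivated when the first enters and OnButtonDeactivated when the last leaves.
; It binds to its own dispatchers to play or reverse a timeline that moves the button's relative Z.
; IsActive reports whether any player is on it.
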(event OnComponentBeginOverlap(Sphere)
  (params (OverlappedComponent :type Primitive%20Component%20Object%20Reference) (OtherActor :type Actor%20Object%20Reference) (OtherComp :type Primitive%20Component%20Object%20Reference) (OtherBodyIndex :type Integer) (bFromSweep :type Boolean) (SweepResult :type Hit%20Result%20Structure%20%28by%20ref%29))
  (bind _charaonbutton (Variables|Default|GetCharaOnButton))
  (bind _asbp_player (Utilities|Casting|CastToBP_Player OtherActor))
  (if (Utilities|Array|IsEmpty _charaonbutton)
    (Default|CallOnButtonActivated self))
  (Utilities|Array|AddUnique _charaonbutton _asbp_player))

(event OnComponentEndOverlap(Sphere)
  (params (OverlappedComponent :type Primitive%20Component%20Object%20Reference) (OtherActor :type Actor%20Object%20Reference) (OtherComp :type Primitive%20Component%20Object%20Reference) (OtherBodyIndex :type Integer))
  (bind _charaonbutton (Variables|Default|GetCharaOnButton))
  (bind _asbp_player (Utilities|Casting|CastToBP_Player OtherActor))
  (Utilities|Array|RemoveItem _charaonbutton _asbp_player)
  (if (Utilities|Array|IsEmpty _charaonbutton)
    (Default|CallOnButtonDeactivated self)))

(event Custom|OnButtonActivated_Event
  (params (Button :type BP%20Button%20Object%20Reference))
  (bind _newtrack_0 (Timeline|ButtonAnim Play)
    (:Update
      (Transformation|SetRelativeLocation (Variables|Default|GetButton) (Math|Vector|MakeVector 0.0 0.0 _newtrack_0) false false))))

(event Custom|OnButtonDeactivated_Event
  (params (Button :type BP%20Button%20Object%20Reference))
  (bind _newtrack_0 (Timeline|ButtonAnim Reverse)
    (:Update
      (Transformation|SetRelativeLocation (Variables|Default|GetButton) (Math|Vector|MakeVector 0.0 0.0 _newtrack_0) false false))))

(event EventBeginPlay
  (EventDispatchers|BindEventtoOnButtonActivated (delegate Custom|OnButtonActivated_Event))
  (EventDispatchers|BindEventtoOnButtonDeactivated (delegate Custom|OnButtonDeactivated_Event)))

(event Collision|EventActorBeginOverlap
  (params (OtherActor :type Actor%20Object%20Reference)))

(event EventTick
  (params (DeltaSeconds :type Float%20%28single-precision%29)))

(fn ConstructionScript)

(fn IsActive
  (return (Utilities|Array|IsNotEmpty (Variables|Default|GetCharaOnButton))))