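; Boat actor that travels between its starting location and an EndPosition actor, driven by a BP_Button child actor.
; On BeginPlay it binds the button events, turns to face the destination and scales the Movement timeline's play rate by TrajectDuration.
; Button activation plays the timeline to interpolate location; deactivation reverses it.
; Both wait DelayBeforeLeaving and recheck the button state before moving.
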(event Custom|OnButtonDeactivated
  (params (Button :type BP%20Button%20Object%20Reference))
  (Utilities|FlowControl|RetriggerableDelay (Variables|Default|GetDelayBeforeLeaving))
  (if (not (Default|IsActive (Variables|Default|GetAs%20BP%20Button)))
    (bind _newtrack_0 (Timeline|Movement Reverse)
      (:Update
        (Transformation|SetActorLocation (+ (Variables|Default|GetStartPosition) (* (- (Transformation|GetActorLocation (Variables|Default|GetEndPosition)) (Variables|Default|GetStartPosition)) _newtrack_0)) false false)))))

(event Custom|OnButtonActivated
  (params (Button :type BP%20Button%20Object%20Reference))
  (Utilities|FlowControl|Delay (Variables|Default|GetDelayBeforeLeaving))
  (if (Default|IsActive (Variables|Default|GetAs%20BP%20Button))
    (bind _newtrack_0 (Timeline|Movement Play)
      (:Update
        (Transformation|SetActorLocation (+ (Variables|Default|GetStartPosition) (* (- (Transformation|GetActorLocation (Variables|Default|GetEndPosition)) (Variables|Default|GetStartPosition)) _newtrack_0)) false false)))))

(event EventBeginPlay
  (bind _asbp_button (Utilities|Casting|CastToBP_Button (Variables|/Script/Engine.ChildActorComponent|GetChildActor (Variables|Default|GetButton))))
  (bind _output_get (Variables|Default|SetAs%20BP%20Button _asbp_button))
  (EventDispatchers|BindEventtoOnButtonActivated _output_get (EventDispatchers|CreateEvent :!event Custom|OnButtonActivated))
  (EventDispatchers|BindEventtoOnButtonDeactivated _output_get (EventDispatchers|CreateEvent :!event Custom|OnButtonDeactivated))
  (Components|Timeline|SetPlayRate (Variables|Default|GetMovement) (/ 1.0 (Variables|Default|GetTrajectDuration)))
  (bind _output_get_2 (Variables|Default|SetStartPosition (Transformation|GetActorLocation)))
  (Transformation|SetActorRotation (Math|Rotator|FindLookatRotation _output_get_2 (Transformation|GetActorLocation (Variables|Default|GetEndPosition)))))

(event Collision|EventActorBeginOverlap
  (params (OtherActor :type Actor%20Object%20Reference)))

(event EventTick
  (params (DeltaSeconds :type Float%20%28single-precision%29)))

(fn ConstructionScript)