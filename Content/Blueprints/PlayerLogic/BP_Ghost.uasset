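; Ghost variant of a parent player Blueprint that replays buffered movement input instead of recording it.
; While running, each tick sums MovementInputBuffer entries timestamped between the last and current elapsed time and applies the result as movement input.
; Empty overrides of AddMovementInputToBuffer and CreateGhost suppress input recording and further ghost creation.
; Death immediately calls StartLife, which resets the replay cursor so the ghost starts over.
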(event EventBeginPlay
  (|CallParentFunction)
  (CallFunction|StartLife))

(event Collision|EventActorBeginOverlap
  (params (OtherActor :type Actor%20Object%20Reference)))

(event EventTick
  (params (DeltaSeconds :type Float%20%28single-precision%29))
  (|CallParentFunction DeltaSeconds)
  (if (Variables|Default|GetIsRunning)
    (Pawn|Input|AddMovementInput (CallFunction|FindInputMovement) 1.0 false)))

(fn ConstructionScript
  (|CallParentFunction))

(fn AddMovementInputtoBuffer
  (params (Input :type Vector :default "0, 0, 0")))

(fn CreateGhost)

(fn FindInputMovement
  (LocalVariables|SetInput "0, 0, 0")
  (bind _keys (Utilities|Map|Keys (Variables|Default|GetMovementInputBuffer)))
  (bind _array_element (Utilities|Array|ForEachLoopwithBreak _keys :!label _label)
    (:LoopBody
      (if (not (< _array_element (Variables|Default|GetLastTimeElapsed)))
        (if (> _array_element (Variables|Default|GetTimeElapsed))
          (goto _label Break)
          (else
            (LocalVariables|SetInput (+ (.Value (Utilities|Map|Find (Variables|Default|GetMovementInputBuffer) _array_element)) (LocalVariables|GetInput)))))))
    (:Completed
      (Variables|Default|SetLastTimeElapsed (Variables|Default|GetTimeElapsed))
      (return (LocalVariables|GetInput)))))

(fn StartLife
  (|CallParentFunction)
  (Variables|Default|SetLastTimeElapsed -1.0))

(fn Die
  (params (DieCause :type E_DieCause%20Enum :default "NewEnumerator0"))
  (|CallParentFunction DieCause)
  (CallFunction|StartLife))