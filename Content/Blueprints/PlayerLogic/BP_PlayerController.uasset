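; Player controller that forwards movement, camera and jump input to the possessed BP_Player.
; BeginPlay caches the controlled pawn, which receives both movement axes through one function with a boolean selecting forward or right.
; Camera axes feed yaw and pitch input straight to the pawn, and jump presses call its jump request.
; A manual pitch-clamp branch using control rotation is present but disconnected, so it never runs.
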(event EventBeginPlay
  (bind _asbp_player (Utilities|Casting|CastToBP_Player (Pawn|GetControlledPawn)))
  (Variables|Default|SetPlayer_BP _asbp_player))

(event EventTick
  (params (DeltaSeconds :type Float%20%28single-precision%29)))

(event Input|ActionEvents|InputActionJump
  (params (Key :type Key%20Structure :default "None"))
  (:Pressed
    (Default|RequestJump (Variables|Default|GetPlayer_BP))))

(event Input|AxisEvents|InputAxisPlayer_Forward
  (params (AxisValue :type Float%20%28single-precision%29))
  (Default|PlayerMovementInput (Variables|Default|GetPlayer_BP) true))

(event Input|AxisEvents|InputAxisPlayer_Right
  (params (AxisValue :type Float%20%28single-precision%29))
  (Default|PlayerMovementInput (Variables|Default|GetPlayer_BP) false))

(event Input|AxisEvents|InputAxisCam_Right
  (params (AxisValue :type Float%20%28single-precision%29))
  (Pawn|Input|AddControllerYawInput (Variables|Default|GetPlayer_BP) AxisValue))

(event Input|AxisEvents|InputAxisCam_Up
  (params (AxisValue :type Float%20%28single-precision%29))
  (Pawn|Input|AddControllerPitchInput (Variables|Default|GetPlayer_BP) AxisValue))

(fn ConstructionScript)