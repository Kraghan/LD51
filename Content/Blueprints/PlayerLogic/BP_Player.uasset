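; Player character for a timed-life ghost mechanic, recording each run's movement and jumps to seed BP_Ghost actors.
; StartLife starts the timer, audio and existing ghosts, while Tick buffers camera-relative, diagonal-corrected input by elapsed time.
; Die, also triggered on timeout, passes start transform, velocity and buffers to a ghost, recycling the oldest at the limit.
; A cause-specific death montage then returns the player to spawn.
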(event Custom|PlayDeath
  (params (DeathType :type E_DieCause%20Enum :default "NewEnumerator0"))
  (switch Utilities|FlowControl|Switch|SwitchonE_DieCause DeathType
    (:NewEnumerator0
      (Animation|Montage|PlayMontage (Variables|Character|GetMesh) "/Game/Anim/AM_DEATH_TIME.AM_DEATH_TIME" :!label _label
        (:OnCompleted
          _)))
    (:NewEnumerator1
      (Animation|Montage|PlayMontage (Variables|Character|GetMesh) "/Game/Anim/AM_DEATH_LAVA.AM_DEATH_LAVA"
        (:OnCompleted
          _)))
    (:NewEnumerator2
      (goto _label)))
  (CallFunction|DeathAnimEnded))

(event EventBeginPlay
  (Variables|Default|SetSpawnTransform (Transformation|GetActorTransform)))

(event Collision|EventActorBeginOverlap
  (params (OtherActor :type Actor%20Object%20Reference)))

(event EventOnJumped
  (Default|CallJumpingStateUpdated "NewEnumerator1"))

(event EventOnLanded
  (params (Hit :type Hit%20Result%20Structure%20%28by%20ref%29))
  (Default|CallJumpingStateUpdated "NewEnumerator3")
  (Variables|Default|SetIsJumping false))

(event EventTick
  (params (DeltaSeconds :type Float%20%28single-precision%29))
  (CallFunction|UpdateLoop DeltaSeconds))

(fn ConstructionScript)

(fn GetControlForward/RightVectors
  (bind _returnvalue (Pawn|GetControlRotation :!class /Script/Engine.Pawn))
  (return (Math|Vector|GetForwardVector (Math|Rotator|MakeRotator 0.0 0.0 (.yaw _returnvalue))) (Math|Vector|GetRightVector (Math|Rotator|MakeRotator 0.0 0.0 (.yaw _returnvalue)))))

(fn PlayerMovementInput
  (params (IsForwardAxis :type Boolean))
  (bind (_forwardvector _rightvector) (CallFunction|GetControlForward/RightVectors))
  (bind _returnvalue (Input|AxisValues|GetPlayer_Forward))
  (bind _returnvalue_2 (Input|AxisValues|GetPlayer_Right))
  (bind (_y_out _x_out) (CallFunction|FixDiagonalGamepadValues _returnvalue _returnvalue_2))
  (if (not (Variables|Default|GetIsDead))
    (if IsForwardAxis
      (Variables|Default|SetCurrentInput (+ (Variables|Default|GetCurrentInput) (* _forwardvector _y_out)))
      (else
        (Variables|Default|SetCurrentInput (+ (Variables|Default|GetCurrentInput) (* _rightvector _x_out)))))))

(fn FixDiagonalGamepadValues
  (params (Y%20in :type Float%20%28double-precision%29) (X%20in :type Float%20%28double-precision%29))
  (return (Math|Float|Clamp(Float) (* Y%20in (Math|Float|MapRangeClamped (Math|Float|Absolute(Float) X%20in) 0.0 0.6 1.0 1.2)) -1.0) (Math|Float|Clamp(Float) (* X%20in (Math|Float|MapRangeClamped (Math|Float|Absolute(Float) Y%20in) 0.0 0.6 1.0 1.2)) -1.0)))

(fn StartLife
  (if (not (Variables|Default|GetIsRunning))
    (Variables|Default|SetIsRunning true)
    (Variables|Default|SetTimeElapse 0.0)
    (Variables|Default|SetStartTransform (Transformation|GetActorTransform))
    (Variables|Default|SetStoredVelocity (Variables|/Script/Engine.MovementComponent|GetVelocity (Variables|Character|GetCharacterMovement)))
    (for _array_element (Variables|Default|GetGhosts)
      (CallFunction|StartLife _array_element))
    (Audio|Components|Audio|Play (Variables|Default|GetAudio) 0.0)))

(fn Die
  (params (DieCause :type E_DieCause%20Enum :default "NewEnumerator0"))
  (if (not (Variables|Default|GetIsDead))
    (Variables|Default|SetIsDead true)
    (CallFunction|CreateGhost)
    (CallFunction|PlayDeath DieCause)
    (Variables|Default|SetIsRunning false)
    (for _array_element (Variables|Default|GetGhosts)
      (CallFunction|Die _array_element "NewEnumerator0"))
    (Audio|Components|Audio|Stop (Variables|Default|GetAudio))))

(fn CreateGhost
  (bind _ghosts (Variables|Default|GetGhosts))
  (bind _starttransform (Variables|Default|GetStartTransform))
  (if (< (Utilities|Array|Length (Variables|Default|GetGhosts)) (Variables|Default|GetGhostLimits))
    (bind _returnvalue (Game|SpawnActorfromClass "/Game/Blueprints/PlayerLogic/BP_Ghost.BP_Ghost_C" (Variables|Default|GetStartTransform) "AlwaysSpawn" 0 0))
    (bind _output_get (LocalVariables|SetGhostToInit _returnvalue))
    (Default|SetColorIndex _output_get (Utilities|Array|Length (Variables|Default|GetGhosts)))
    (else
      (bind _output_get_2 (LocalVariables|SetGhostToInit (Utilities|Array|Get(acopy) _ghosts)))
      (Transformation|SetActorLocationAndRotation _output_get_2 (.location _starttransform) (.rotation _starttransform))
      (Variables|BP_Player_C|SetSpawnTransform _output_get_2 (Variables|Default|GetStartTransform))
      (Utilities|Array|RemoveIndex _ghosts)))
  (Utilities|Array|Add (Variables|Default|GetGhosts) (LocalVariables|GetGhostToInit))
  (Variables|BP_Player_C|SetMovementInputsBuffer (LocalVariables|GetGhostToInit) (Variables|Default|GetMovementInputsBuffer))
  (Utilities|Map|Clear (Variables|Default|GetMovementInputsBuffer))
  (Variables|/Game/Blueprints/PlayerLogic/BP_Ghost.BP_Ghost_C|SetInitialVelocity (LocalVariables|GetGhostToInit) (Variables|Default|GetStoredVelocity))
  (Variables|BP_Player_C|SetJumpRequests (LocalVariables|GetGhostToInit) (Variables|Default|GetJumpRequests))
  (Utilities|Array|Clear (Variables|Default|GetJumpRequests)))

(fn DeathAnimEnded
  (bind _spawntransform (Variables|Default|GetSpawnTransform))
  (Transformation|SetActorLocation (.location _spawntransform) false false)
  (Transformation|SetActorRotation (.rotation _spawntransform))
  (Variables|Default|SetIsDead false))

(fn AddMovementInputtoBuffer
  (params (Input :type Vector))
  (if (Variables|Default|GetIsRunning)
    (Utilities|Map|Add (Variables|Default|GetMovementInputsBuffer) (Variables|Default|GetTimeElapse) Input)))

(fn RequestJump
  (if (not (Variables|Default|GetIsDead))
    (Default|CallJumpingStateUpdated "NewEnumerator0")
    (Variables|Default|SetIsJumping true)
    (Utilities|Array|Add (Variables|Default|GetJumpRequests) (Variables|Default|GetTimeElapse))))

(fn Debug)

(fn UpdateJumpState
  (if (Variables|Default|GetIsJumping)
    (if (and (not (Variables|Default|GetWasFalling)) (AI|Components|NavMovement|IsFalling (Variables|Character|GetCharacterMovement)))
      (Default|CallJumpingStateUpdated "NewEnumerator2")))
  (Variables|Default|SetWasFalling (AI|Components|NavMovement|IsFalling (Variables|Character|GetCharacterMovement))))

(fn UpdateTimer
  (params (DeltaTime :type Float%20%28double-precision%29))
  (bind _output_get (Variables|Default|SetTimeElapse (+ (Variables|Default|GetTimeElapse) DeltaTime)))
  (Development|PrintString (Utilities|String|ToString(Float) (- (Variables|Default|GetLifeTime) _output_get)) true true (Math|Conversions|ToLinearColor(Color) (Variables|Default|GetColor)) 0.0)
  (if (>= _output_get (Variables|Default|GetLifeTime))
    (CallFunction|Die "NewEnumerator0")))

(fn UpdateMovement
  (CallFunction|AddMovementInputtoBuffer (Variables|Default|GetCurrentInput))
  (Pawn|Input|AddMovementInput (Math|Vector|Normalize (Variables|Default|GetCurrentInput)) (Math|Vector|VectorLength (Variables|Default|GetCurrentInput)) false)
  (Variables|Default|SetCurrentInput "0, 0, 0"))

(fn UpdateLoop
  (params (DeltaTime :type Float%20%28double-precision%29))
  (CallFunction|UpdateJumpState)
  (if (Variables|Default|GetIsRunning)
    (CallFunction|UpdateTimer DeltaTime)
    (else
      (if (Utilities|Operators|EqualEqual :A (Pawn|Components|PawnMovement|GetLastInputVector (Variables|Character|GetCharacterMovement)))
        _
        (else
          _))
      (Development|PrintString "Waiting start" true true "(R=0.000000,G=0.660000,B=1.000000,A=1.000000)" 0.0)))
  (CallFunction|UpdateMovement)
  (return))